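; BP_ATPlayerState is a player state Blueprint that holds the player's HP values and counts uses of three consumables: liquor, rocks and smoke shells.
; Each Consume event calls its matching Used function, which increments that item's counter.
; BeginPlay calls InitMyState with the state's own CurrentHP and MaxHP, so the initialization writes the same values back.
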(event EventConsumeLiquor
  (CallFunction|UsedLiquor))

(event EventConsumeRock
  (CallFunction|UsedRock))

(event EventConsumeSmokeShell
  (CallFunction|UsedSmoekShell))

(event EventBeginPlay
  (CallFunction|InitMyState (Variables|Default|GetCurrentHP) (Variables|Default|GetMaxHP)))

(fn ConstructionScript)

(fn UsedLiquor
  (Math|Integer|IncrementInt (Variables|Default|GetLiquorCount)))

(fn UsedSmoekShell
  (Math|Integer|IncrementInt (Variables|Default|GetSmokeShellCount)))

(fn UsedRock
  (Math|Integer|IncrementInt (Variables|Default|GetRockCount)))

(fn InitMyState
  (params (CurrentHP :type Float%20%28single-precision%29) (MaxHP :type Float%20%28single-precision%29))
  (Variables|Default|SetCurrentHP CurrentHP)
  (Variables|Default|SetMaxHP MaxHP))
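; AI controller for the ranged enemy, running BT_RangedTree from BeginPlay.
; Perception updates pass each actor to CheckPlayer, which toggles PlayerActorKey for PLAYER-tagged actors: it clears the key if already valid, otherwise stores the actor, printing Lost or Sensed.
; The toggle infers gain or loss from blackboard state alone, without reading the stimulus.
; A RockLocation event sets the focal point to a given position and writes it to the blackboard.
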(event OnPerceptionUpdated(AIPerception)
  (params (UpdatedActors :type Array%20of%20Actor%20Object%20References))
  (for _array_element UpdatedActors
    (CallFunction|CheckPlayer _array_element)))

(event EventBeginPlay
  (AI|RunBehaviorTree "/Game/EnemyAI/RangedAI/BT_RangedTree.BT_RangedTree"))

(event EventRockLocation
  (params (Rock :type Vector :default "0, 0, 0"))
  (AI|SetFocalPoint Rock)
  (AI|Components|Blackboard|SetValueasVector (AI|GetBlackboard 0) (Utilities|Name|MakeLiteralName "RockLocation") Rock))

(fn ConstructionScript)

(fn CheckPlayer
  (params (SensedPlayer :type Actor%20Object%20Reference))
  (if (Actor|ActorHasTag SensedPlayer "PLAYER")
    (Utilities|IsValid (AI|Components|Blackboard|GetValueasObject (AI|GetBlackboard 0) (Utilities|Name|MakeLiteralName "PlayerActorKey"))
      (:Is%20Valid
        (AI|Components|Blackboard|SetValueasObject (AI|GetBlackboard 0) (Utilities|Name|MakeLiteralName "PlayerActorKey") 0)
        (Development|PrintString "Lost" true true "(R=1.000000,G=0.252799,B=0.000000,A=1.000000)" 5.0))
      (:Is%20Not%20Valid
        (AI|Components|Blackboard|SetValueasObject (AI|GetBlackboard 0) (Utilities|Name|MakeLiteralName "PlayerActorKey") SensedPlayer)
        (Development|PrintString "Sensed" true true "(R=0.081855,G=1.000000,B=0.386039,A=1.000000)" 5.0)))))
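; BP_RangedCharacter is a ranged AI enemy that investigates perceived stimuli and attacks by throwing.
; On BeginPlay it focuses on BPPoint and stores it as the blackboard's origin point.
; Perception updates set or clear the investigating key, and successful senses send the stimulus location to the controller through RockLocationMessage.
; Separate events play the throw montage and spawn a scaled-up BP_Throwing projectile at the SpawnWeapon component, facing the actor's rotation.
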(event OnTargetPerceptionUpdated(AIPerception)
  (params (Actor :type Actor%20Object%20Reference) (Stimulus :type AI%20Stimulus%20Structure))
  (bind (_age _expirationage _strength _stimuluslocation _receiverlocation _tag _bsuccessfullysensed) (Utilities|Struct|BreakAIStimulus Stimulus))
  (bind _returnvalue (AI|GetBlackboard 0))
  (bind _returnvalue_2 (Utilities|Name|MakeLiteralName "investigating?"))
  (if _bsuccessfullysensed
    (bind _output_get (Variables|Default|Setinvestigating? _bsuccessfullysensed))
    (AI|Components|Blackboard|SetValueasBool _returnvalue _returnvalue_2 _output_get)
    (Class|BPIRnage|RockLocation(Message) (Pawn|GetController) _stimuluslocation)
    (else
      (AI|Components|Blackboard|ClearValue _returnvalue _returnvalue_2))))

(event Custom|Spawn%20Weapon
  (Game|SpawnActorfromClass "/Game/EnemyAI/RangedAI/BP_Throwing.BP_Throwing_C" (Math|Transform|MakeTransform (Transformation|GetWorldLocation (Variables|Default|GetSpawnWeapon)) (Transformation|GetActorRotation) "2.000000,2.000000,2.000000") "Undefined" 0 0))

(event EventBeginPlay
  (bind _bp_point (Variables|Default|GetBP_Point))
  (AI|SetFocus (AI|GetAIController self) _bp_point)
  (AI|Components|Blackboard|SetValueasObject (AI|GetBlackboard 0) (Utilities|Name|MakeLiteralName "OriginPointKey") _bp_point))

(event EventRangeAttack
  (Animation|PlayAnimMontage "/Game/EnemyAI/RangedAI/Animation/ThrowAttack_Montage.ThrowAttack_Montage" 2.0 "None"))

(fn ConstructionScript)